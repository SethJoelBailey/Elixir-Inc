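; BP_QuestLogic selects a random quest that the player's Fame qualifies for.
; SelectQuest loops over the CompQuests quest list and adds entries whose NeededFame is below the first-person character's Fame to ValidQuests, without clearing that array first.
; It returns customer name, base gold reward and description through random picks from ValidQuests.
; The event graph and construction script are empty.
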(event EventBeginPlay)

(event EventTick
  (params (DeltaSeconds :type Float%20%28single-precision%29)))

(fn ConstructionScript)

(fn SelectQuest
  (bind _comp_quests (Variables|Default|GetComp_Quests))
  (bind _validquests (LocalVariables|GetValidQuests))
  (bind _outitem (Utilities|Array|Random _validquests))
  (bind _questlist (Variables|/Game/Quests/Comp_Quests.Comp_Quests_C|GetQuestList _comp_quests))
  (bind _asbp_first_person_character (Utilities|Casting|CastToBP_FirstPersonCharacter (Game|GetPlayerCharacter 0)))
  (for (_array_element _array_index) _questlist
    (if (> (Variables|/Game/FirstPerson/Blueprints/BP_FirstPersonCharacter.BP_FirstPersonCharacter_C|GetFame _asbp_first_person_character) (.neededfame _array_element))
      (Utilities|Array|Add (LocalVariables|GetValidQuests) (Utilities|Array|Get(acopy) _questlist _array_index))))
  (return (.customername _outitem) (.basegold _outitem) (.questdescription _outitem)))