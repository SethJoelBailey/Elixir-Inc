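; BP_DimensionShiftPotion is a collectable potion that alters the level when picked up.
; On BeginPlay it registers its potion through CompDesignatedPotion.
; Interaction loops over potions of its class but returns in the first iteration, marking that one discovered, collecting and destroying itself.
; It also brightens the DirectionalLight, reveals BP_PlaceholderShpere actors with collision, and zeroes the BP_TransmutationLight intensity.
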(event EventBeginPlay
  (bind _comp_designatedpotion (Variables|Default|GetComp_DesignatedPotion))
  (Default|AddtoPotionList _comp_designatedpotion (Variables|/Game/Potions/Comp_DesignatedPotion.Comp_DesignatedPotion_C|GetPotion _comp_designatedpotion)))

(event Collision|EventActorBeginOverlap
  (params (OtherActor :type Actor%20Object%20Reference)))

(event EventTick
  (params (DeltaSeconds :type Float%20%28single-precision%29)))

(fn ConstructionScript)

(fn Interaction
  (bind _outactors (Actor|GetAllActorsOfClass "BP_DimensionShiftPotion_C"))
  (for _array_element _outactors
    (Variables|BP_DimensionShiftPotion_C|SetHasBeenDiscovered _array_element true)
    (Default|GetCollected (Variables|Default|GetComp_Collectable))
    (Actor|DestroyActor)
    (bind _returnvalue (Actor|GetActorOfClass "/Script/Engine.DirectionalLight"))
    (Rendering|Components|Light|SetIntensity (Variables|/Script/Engine.Light|GetLightComponent _returnvalue) 1e+01)
    (bind _outactors_2 (Actor|GetAllActorsOfClass "/Game/Transmutation/BP_PlaceholderShpere.BP_PlaceholderShpere_C"))
    (for _array_element_2 _outactors_2
      (Rendering|SetActorHiddenInGame _array_element_2 false)
      (Collision|SetActorEnableCollision _array_element_2 true))
    (bind _returnvalue_2 (Actor|GetActorOfClass "/Game/Transmutation/BP_TransmutationLight.BP_TransmutationLight_C"))
    (Rendering|Components|Light|SetIntensity (Variables|/Game/Transmutation/BP_TransmutationLight.BP_TransmutationLight_C|GetPointLight _returnvalue_2) 0.0)
    (return true)))