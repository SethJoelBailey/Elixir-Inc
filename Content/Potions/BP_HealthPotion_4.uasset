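; Health potion pickup actor, one of a numbered set, that registers its potion with its designated-potion component on BeginPlay.
; Its Interaction function only fetches all BP_HealthPotion actors and does nothing with the result.
; The pickup logic is disconnected and never runs: collect and destroy, brighten the directional light, reveal placeholder spheres and switch off the transmutation light.
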(event EventBeginPlay
  (bind _comp_designatedpotion (Variables|Default|GetComp_DesignatedPotion))
  (Default|AddtoPotionList _comp_designatedpotion (Variables|/Game/Potions/Comp_DesignatedPotion.Comp_DesignatedPotion_C|GetPotion _comp_designatedpotion)))

(event Collision|EventActorBeginOverlap
  (params (OtherActor :type Actor%20Object%20Reference)))

(event EventTick
  (params (DeltaSeconds :type Float%20%28single-precision%29)))

(fn ConstructionScript)

(fn Interaction
  (Actor|GetAllActorsOfClass "/Game/Potions/BP_HealthPotion.BP_HealthPotion_C"))