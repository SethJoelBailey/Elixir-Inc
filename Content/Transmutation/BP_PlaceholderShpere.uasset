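; Placeholder sphere actor that marks a transmutation spot and opens the inventory when interacted with.
; Interaction does its work only if no inventory widget is open, creating one and switching to cursor-driven Game and UI input.
; It then passes its transform and location to the first-person character, increments TransmutationCount and enables item placement.
; The sphere also hides, disables collision and tags itself "Selected".
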(event EventBeginPlay)

(event Collision|EventActorBeginOverlap
  (params (OtherActor :type Actor%20Object%20Reference)))

(event EventTick
  (params (DeltaSeconds :type Float%20%28single-precision%29)))

(fn ConstructionScript)

(fn Interaction
  (bind _returnvalue (Game|GetPlayerController 0))
  (bind _foundwidgets (Widget|GetAllWidgetsOfClass "/Game/Inventory/W_Inventory.W_Inventory_C" true))
  (Utilities|IsValid (Utilities|Array|Get(acopy) _foundwidgets)
    (:Is%20Not%20Valid
      (bind _returnvalue_2 (UserInterface|CreateWidget "/Game/Inventory/W_Inventory.W_Inventory_C"))
      (UserInterface|Viewport|AddtoViewport _returnvalue_2 0)
      (Input|SetInputModeGameandUI _returnvalue 0 "DoNotLock" true)
      (Variables|/Script/Engine.PlayerController|SetbShowMouseCursor _returnvalue true)
      (bind _asbp_first_person_character (Utilities|Casting|CastToBP_FirstPersonCharacter (Game|GetPlayerCharacter 0)))
      (Variables|/Game/FirstPerson/Blueprints/BP_FirstPersonCharacter.BP_FirstPersonCharacter_C|SetTransmutationSphereLocation _asbp_first_person_character (Transformation|GetActorTransform))
      (Variables|/Game/FirstPerson/Blueprints/BP_FirstPersonCharacter.BP_FirstPersonCharacter_C|SetTransmutationCount _asbp_first_person_character (+ (Variables|/Game/FirstPerson/Blueprints/BP_FirstPersonCharacter.BP_FirstPersonCharacter_C|GetTransmutationCount _asbp_first_person_character) 1))
      (Rendering|SetActorHiddenInGame true)
      (Collision|SetActorEnableCollision false)
      (Variables|/Game/FirstPerson/Blueprints/BP_FirstPersonCharacter.BP_FirstPersonCharacter_C|SetCanItemBePlaced _asbp_first_person_character true)
      (Variables|/Game/FirstPerson/Blueprints/BP_FirstPersonCharacter.BP_FirstPersonCharacter_C|SetSphereVector _asbp_first_person_character (Transformation|GetActorLocation))
      (Variables|Default|SetTags (Utilities|Array|MakeArray "Selected"))
      (return true))))