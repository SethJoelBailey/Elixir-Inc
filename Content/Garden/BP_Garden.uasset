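; BP_Garden is a garden actor that scatters random herb ingredient actors around its bounds origin when play begins.
; SpawnWithinRange loops on the NumberOfIngrediants counter, picking one of six ingredient classes each pass, then resets the counter.
; Spawns use random XY offsets in a fixed square with a slight Z lift, adjusting for collisions but always spawning.
; The bounds extent is passed as Area but never used.
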(event EventBeginPlay
  (bind _self self)
  (bind (_origin _boxextent) (Collision|GetActorBounds _self false false))
  (CallFunction|SpawnWithinRange _boxextent (Math|Conversions|ToTransform(Vector) _origin)))

(event Collision|EventActorBeginOverlap
  (params (OtherActor :type Actor%20Object%20Reference)))

(event EventTick
  (params (DeltaSeconds :type Float%20%28single-precision%29)))

(fn ConstructionScript)

(fn SpawnWithinRange
  (params (Area :type Vector) (Oirgin :type Transform))
  (bind _output_get (LocalVariables|SetIngrediantArray (Utilities|Array|MakeArray "/Game/Ingrediants/Ingrediant_Borage.Ingrediant_Borage_C" "/Game/Ingrediants/Ingrediant_Verbascum.Ingrediant_Verbascum_C" "/Game/Ingrediants/Ingrediant_RedSage.Ingrediant_RedSage_C" "/Game/Ingrediants/Ingrediant_Eyebright.Ingrediant_Eyebright_C" "/Game/Ingrediants/Ingrediant_Aralia.Ingrediant_Aralia_C" "/Game/Ingrediants/Ingrediant_Sorrel.Ingrediant_Sorrel_C") :!label _label))
  (Game|SpawnActorfromClass (.OutItem (Utilities|Array|Random _output_get)) (Math|Conversions|ToTransform(Vector) (Math|Transform|TransformLocation Oirgin (+ (Math|Vector|MakeVector (Math|Random|RandomFloatinRange -5.5e+02 5.5e+02) (Math|Random|RandomFloatinRange -5.5e+02 5.5e+02) 0.0) "0,0,40.000000"))) "AdjustIfPossibleButAlwaysSpawn" 0 0)
  (Variables|Default|SetNumberOfIngrediants (- (Variables|Default|GetNumberOfIngrediants) 1))
  (if (> (Variables|Default|GetNumberOfIngrediants) 0)
    (goto _label)
    (else
      (Variables|Default|SetNumberOfIngrediants 10))))